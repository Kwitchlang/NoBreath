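; LightBP is a flickering light fixture pairing a rect light with a static mesh whose material glows.
; Construction sets the light to its configured intensity; on BeginPlay it creates a dynamic LightFlicker material and loops indefinitely on short random delays.
; Each pass randomizes the light intensity and the material's Intensity parameter, remapped to a smaller range.
; Light and material evaluate their random values separately, so their brightness need not match.
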(event `self.ReceiveBeginPlay`
  (bind _returnvalue (`KismetMathLibrary.RandomFloatInRange` 0.0 1200.0))
  (bind _returnvalue_2 (`PrimitiveComponent.CreateDynamicMaterialInstance` (`self.StaticMesh`) 1 "/Game/Materials/LightFlicker.LightFlicker" "None"))
  (`LightComponent.SetIntensity` (`self.RectLight`) _returnvalue :!label _label)
  (`MaterialInstanceDynamic.SetScalarParameterValue` _returnvalue_2 "Intensity" (`KismetMathLibrary.MapRangeClamped` _returnvalue 0.0 1200.0 0.0 10.0))
  (`KismetSystemLibrary.Delay` (`KismetMathLibrary.RandomFloatInRange` 0.0 0.3))
  (goto _label))

(fn `UserConstructionScript`
  (`LightComponent.SetIntensity` (`self.RectLight`) (`self.Light Intensity`)))