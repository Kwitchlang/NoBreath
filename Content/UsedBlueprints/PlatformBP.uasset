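; Moving platform Blueprint that, once activated through ActivateObject, travels between relative waypoints in LocationArray.
; Tick moves the Platform component with constant-speed interpolation using a fixed DeltaTime of 1.0, so speed depends on frame rate.
; On arrival it waits a Delay, then picks the next waypoint by SwitchMethod: stop at the last, loop to the first, or ping-pong.
; The keycard and teleport-blocker query functions return only fixed defaults.
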(event `self.ReceiveTick`
  (params (DeltaSeconds :type "Float (single-precision)"))
  (bind _location_array (`self.Location Array`))
  (bind _location_select (`self.Location Select`))
  (bind _platform (`self.Platform`))
  (bind _returnvalue (- (`self.Location Select`) 1))
  (bind _returnvalue_2 (+ _location_select 1))
  (bind _output (`|GetArrayItem` _location_array (`self.Location Select`)))
  (bind _relativelocation (`SceneComponent.RelativeLocation` _platform))
  (if (`self.Exe Activate`)
    (if (`KismetArrayLibrary.Array_IsValidIndex` _location_array 1)
      (`SceneComponent.K2_SetRelativeLocation` _platform (`KismetMathLibrary.VInterpTo_Constant` _relativelocation _output 1.0 (`self.Interp Speed`)) false false)
      (if (== _relativelocation _output :`ErrorTolerance` 0.001)
        (bind _output_get (set `self.Location == Target` true))
        (if _output_get
          (set `self.Location == Target` false)
          (`KismetSystemLibrary.Delay` (`self.Delay`))
          (switch `/Game/Blueprints/MultifacetPanel/method` (`self.SwitchMethod`)
            (:`NewEnumerator0`
              (set `self.Location Select` (`KismetMathLibrary.Clamp` (+ (`self.Location Select`) 1) 0 (`KismetArrayLibrary.Array_LastIndex` (`self.Location Array`)))))
            (:`NewEnumerator2`
              (if (> (+ (`self.Location Select`) 1) (`KismetArrayLibrary.Array_LastIndex` (`self.Location Array`)))
                (set `self.Location Select` 0)
                (else
                  (set `self.Location Select` (+ (`self.Location Select`) 1)))))
            (:`NewEnumerator1`
              (if (`self.Backwards`)
                (if (< _returnvalue 0)
                  (set `self.Backwards` false)
                  (set `self.Location Select` (+ (`self.Location Select`) 1))
                  (else
                    (set `self.Location Select` _returnvalue)))
                (elif (> _returnvalue_2 (`KismetArrayLibrary.Array_LastIndex` (`self.Location Array`)))
                  (set `self.Backwards` true)
                  (set `self.Location Select` (- _location_select 1))
                  (else
                    (set `self.Location Select` _returnvalue_2)))))))))))

(event `Activate Object`
  (set `self.Exe Activate` true :!label _label))

(event `/Game/Blueprints/Systems/PlayerInterface.ActivateObject`
  (goto _label))

(fn `Return keycard Object`
  (returns (`Keycard Level` :type "/Game/Blueprints/Keycard/keycardAccessLevel Enum") (Executed :type Boolean))
  (return "NewEnumerator0" false))

(fn `Return Teleport Through Blocker`
  (returns (`IS valid Object` :type Boolean))
  (return false))

(fn `UserConstructionScript`)