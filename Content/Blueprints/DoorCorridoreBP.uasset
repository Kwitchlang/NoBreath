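; A corridor door that opens while something overlaps its Detection volume, but only once it has been activated.
; Activation, either preset or through AuthorityActivateObject, enables query collision on Detection; otherwise collision is disabled at BeginPlay.
; Tick pushes the open state to the door's Animation Blueprint and blends a dynamic emissive material's color via HSV lerp, green when active, red when inactive.
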(event `self.ReceiveTick`
  (params (DeltaSeconds :type "Float (single-precision)"))
  (bind _material_instance (`self.Material Instance`))
  (`|ExecutionSequence`
    (:`then_0`
      (if (`self.Activate From player`)
        (set `self.NewVar_0` (struct :`R` 0.024614 :`G` 0.265012 :`A` 1.0))
        (else
          (set `self.NewVar_0` (struct :`R` 1.0 :`B` 0.013553 :`A` 1.0)))))
    (:`then_1`
      (`self.Set Animation Variable` (`self.Door State Open`))
      (bind _returnvalue (`MaterialInstanceDynamic.K2_GetVectorParameterValue` _material_instance "Color"))
      (`MaterialInstanceDynamic.SetVectorParameterValue` _material_instance "Color" (`KismetMathLibrary.LinearColorLerpUsingHSV` _returnvalue (`self.NewVar_0`) (* DeltaSeconds 3.0))))))

(event `/Game/Blueprints/Systems/Interfaces/AuthoritiveInterface.Authority Activate Object`
  (set `self.Activate From player` true)
  (`PrimitiveComponent.SetCollisionEnabled` (`self.Detection`) "QueryOnly"))

(event `self.ReceiveBeginPlay`
  (bind _returnvalue (`PrimitiveComponent.CreateDynamicMaterialInstance` (`self.Door Mesh`) 4 "/Game/Assets/Materials/CorridoreMaterials/GlowEmmisiveINST.GlowEmmisiveINST" "None"))
  (set `self.Material Instance` _returnvalue)
  (if (`self.Activate From player`)
    (set `self.Activate From player` true)
    (`PrimitiveComponent.SetCollisionEnabled` (`self.Detection`) "QueryOnly")
    (else
      (`ActorComponent.SetActive` (`self.Detection`) false false)
      (`PrimitiveComponent.SetCollisionEnabled` (`self.Detection`) "NoCollision"))))

(event `self.Detection.OnComponentBeginOverlap`
  (params (OverlappedComponent :type "PrimitiveComponent Object Reference") (OtherActor :type "Actor Object Reference") (OtherComp :type "PrimitiveComponent Object Reference") (OtherBodyIndex :type Integer) (bFromSweep :type Boolean) (SweepResult :type "HitResult Structure (by ref)"))
  (set `self.Door State Open` true))

(event `self.Detection.OnComponentEndOverlap`
  (params (OverlappedComponent :type "PrimitiveComponent Object Reference") (OtherActor :type "Actor Object Reference") (OtherComp :type "PrimitiveComponent Object Reference") (OtherBodyIndex :type Integer))
  (set `self.Door State Open` false))

(fn `Set Animation Variable`
  (params (`Open ` :type Boolean))
  (`|ExecutionSequence`
    (:`then_0`
      (bind _asdoor__animation_bp (cast `/Game/Assets/CorridoreMesh/ScifiDoors/Door-AnimationBP` (`SkeletalMeshComponent.GetAnimInstance` (`self.Door Mesh`))))
      (set `/Game/Assets/CorridoreMesh/ScifiDoors/Door-AnimationBP.Open ` `Open ` _asdoor__animation_bp))))

(fn `UserConstructionScript`
  (`|ExecutionSequence`
    (:`then_0`
      (`self.Set Animation Variable` (`self.Door State Open`)))))