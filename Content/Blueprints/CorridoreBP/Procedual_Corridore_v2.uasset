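; Procedural corridor prototype Blueprint that edits the points of a spline; it places no meshes yet.
; GeneratePoints appends a point offset a fixed distance along local X from the spline's end.
; RemovePoints loops upward from index 1 removing points while indices shift, so it may not clear them all.
; The construction script only prints the spline length, and some leftover nodes are disconnected.
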(event `Generate Points`
  (bind _spline (`self.Spline`))
  (bind _returnvalue (`SplineComponent.GetNumberOfSplinePoints` _spline))
  (`SplineComponent.AddSplinePointAtIndex` _spline (+ (`SplineComponent.GetLocationAtSplinePoint` _spline _returnvalue "Local") (300.0 0.0 0.0)) _returnvalue "Local" true))

(event `Remove Points`
  (for _index (range 1 (+ (`SplineComponent.GetNumberOfSplinePoints` (`self.Spline`)) 1))
    (`SplineComponent.RemoveSplinePoint` (`self.Spline`) _index true)))

(fn `UserConstructionScript`
  (`KismetSystemLibrary.PrintString` (`KismetStringLibrary.Conv_DoubleToString` (`SplineComponent.GetSplineLength` (`self.Spline`)))))