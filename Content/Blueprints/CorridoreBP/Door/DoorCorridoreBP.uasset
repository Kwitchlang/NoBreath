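; Corridor door Blueprint that opens and closes automatically when something overlaps its Detection volume, once unlocked.
; ActivateObject or an initially unlocked state enables Detection collision; locked doors disable it on BeginPlay.
; Overlap events set DoorStateOpen, which Tick and the construction script pass to the door's animation Blueprint.
; OpenCloseDoor toggles the state manually, while keycard, environment and teleport queries return fixed defaults.
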(event `self.ReceiveTick`
  (params (DeltaSeconds :type "Float (single-precision)"))
  (`self.Set Animation Variable` (`self.Door State Open`))
  (if (`self.Unlocked`)
    _))

(event `/Game/Blueprints/Systems/PlayerInterface.ActivateObject`
  (set `self.Unlocked` true)
  (`PrimitiveComponent.SetCollisionEnabled` (`self.Detection`) "QueryOnly"))

(event `self.ReceiveBeginPlay`
  (if (`self.Unlocked`)
    (set `self.Unlocked` true)
    (`PrimitiveComponent.SetCollisionEnabled` (`self.Detection`) "QueryOnly")
    (else
      (`ActorComponent.SetActive` (`self.Detection`) false false)
      (`PrimitiveComponent.SetCollisionEnabled` (`self.Detection`) "NoCollision"))))

(event `Open Close Door`
  (bind _isa (`/Engine/EditorBlueprintResources/StandardMacros.FlipFlop`)
    (:`A`
      _)
    (:`B`
      _))
  (bind _output_get (set `self.Door State Open` _isa))
  (`self.Set Animation Variable` _output_get))

(event `self.Detection.OnComponentBeginOverlap`
  (params (OverlappedComponent :type "PrimitiveComponent Object Reference") (OtherActor :type "Actor Object Reference") (OtherComp :type "PrimitiveComponent Object Reference") (OtherBodyIndex :type Integer) (bFromSweep :type Boolean) (SweepResult :type "HitResult Structure (by ref)"))
  (set `self.Door State Open` true))

(event `self.Detection.OnComponentEndOverlap`
  (params (OverlappedComponent :type "PrimitiveComponent Object Reference") (OtherActor :type "Actor Object Reference") (OtherComp :type "PrimitiveComponent Object Reference") (OtherBodyIndex :type Integer))
  (set `self.Door State Open` false))

(fn ` Is Enviroment NOT Safe`
  (returns (`Not safe?` :type Boolean))
  (return false))

(fn `Return keycard Object`
  (returns (`Keycard Level` :type Byte) (Executed :type Boolean))
  (return 0 true))

(fn `Return Teleport Through Blocker`
  (returns (`IS valid Object` :type Boolean))
  (return false))

(fn `Set Animation Variable`
  (params (`Open ` :type Boolean))
  (bind _asdoor__animation_bp (cast `/Game/Blueprints/CorridoreBP/Door/Door-AnimationBP` (`SkeletalMeshComponent.GetAnimInstance` (`self.Door Mesh`))))
  (set `/Game/Blueprints/CorridoreBP/Door/Door-AnimationBP.Open ` `Open ` _asdoor__animation_bp))

(fn `UserConstructionScript`
  (`self.Set Animation Variable` (`self.Door State Open`)))