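; PocketLog is an interactable pickup actor that adds a readable data entry to the player's log.
; When activated while its player line-trace flag is set, it passes its data struct to the GameInstance's log UI, then destroys itself.
; Notes, personal logs and security details also display on screen immediately, while emails are only logged.
; Its content and interactive-type query functions return only default values.
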(event `/Game/Blueprints/Systems/Interfaces/PlayerInteractableInterface.Activate Object`
  (bind _custome_game_instance (`/Game/Blueprints/Systems/SystemFunctionLibrary.Game Instance Pure`))
  (bind _data_struct (`self.Data Struct`))
  (if (`self.Linetrace connecting with player`)
    (`|ExecutionSequence`
      (:`then_0`
        (switch `/Game/Blueprints/InteractableCLASS/DataObjectType` (`self.Data type`)
          (:`NewEnumerator0`
            (`/Game/Blueprints/Systems/CustomgameInstance.Display UI to Screen` _custome_game_instance _data_struct :!label _label))
          (:`NewEnumerator1`
            _)
          (:`NewEnumerator2`
            (goto _label))
          (:`NewEnumerator3`
            (goto _label)))
        (`/Game/Blueprints/Systems/CustomgameInstance.Add Entry to Log UI` _custome_game_instance _data_struct))
      (:`then_1`
        (`self.K2_DestroyActor`)))))

(fn `Return Interactive Type`
  (returns (NewParam :type "/Game/Blueprints/InteractableCLASS/InteractableType Enum") (NewParam :type "/Game/Blueprints/InteractableCLASS/InteractableType Enum"))
  (return "NewEnumerator0" "NewEnumerator0"))

(fn `Return PocketLog Contents`
  (returns (Contents :type "/Game/Blueprints/StructsEnums/DataStruct Structure") (Contents_To :type Text) (Contents_From :type Text) (Contents_Subject :type Text) (Contents_Contents :type Text) (Contents :type "/Game/Blueprints/StructsEnums/DataStruct Structure") (Contents_To :type Text) (Contents_From :type Text) (Contents_Subject :type Text) (Contents_Contents :type Text))
  (return (make `/Game/Blueprints/StructsEnums/DataStruct` "") "" "" "" "" (make `/Game/Blueprints/StructsEnums/DataStruct` "") "" "" "" ""))

(fn `UserConstructionScript`)