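; TerminalBP is a terminal Blueprint that displays an interactive-style button menu through a Widget component.
; On BeginPlay it creates a TerminalUI with a reference to itself, assigns it to the component, then adds one ButtonUI per TerminalButtons struct entry, printing each index.
; Functions for keycard lookup and teleporting through blockers return only fixed defaults, and the construction script is empty.
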(event `self.ReceiveBeginPlay`
  ;[1 1 1] Set up UI
  (bind _returnvalue (`|CreateWidget` "/Game/Blueprints/Terminal/TerminalUI.TerminalUI_C" null self))
  (bind _output_get (set `self.Terminal UI` _returnvalue))
  (`WidgetComponent.SetWidget` (`self.Widget`) _output_get)
  (for (_array_element _array_index) (`self.TerminalButtons`)
    (`KismetSystemLibrary.PrintString` (`KismetStringLibrary.Concat_StrStr` "attach: " (`KismetStringLibrary.Conv_IntToString` _array_index)))
    (bind _returnvalue_2 (`|CreateWidget` "/Game/Blueprints/Terminal/ButtonUI.ButtonUI_C" null _array_element))
    (`PanelWidget.AddChild` (`/Game/Blueprints/Terminal/TerminalUI.Buttons` (`self.Terminal UI`)) _returnvalue_2)))

(fn `Return keycard Object`
  (returns (`Keycard Level` :type "/Game/Blueprints/Keycard/keycardAccessLevel Enum") (Executed :type Boolean))
  (return "NewEnumerator0" false))

(fn `Return Teleport Through Blocker`
  (returns (`IS valid Object` :type Boolean))
  (return false))

(fn `UserConstructionScript`)