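; Keycard-gated terminal actor that shows a TerminalUI screen linked to a designated ActivateObject.
; On BeginPlay it creates the UI with that object and assigns it to its widget component.
; SendPlayerKeys checks received keycards against RequiredKeys to set AllowAction, while getters report it as non-blocking and return its keycard object type.
; The construction script moves a spline point to ActivateObject, visually linking the two.
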(event `self.ReceiveBeginPlay`
  (bind _returnvalue (`|CreateWidget` "/Game/UI/TerminalUI.TerminalUI_C" null (`self.Activate Object`)))
  (`WidgetComponent.SetWidget` (`self.Widget`) _returnvalue))

(event `/Game/Blueprints/Systems/PlayerInterface.Send Player Keys`
  (params (`Player keycards` :type "Map of /Game/Blueprints/Keycard/keycardAccessLevel Enum to Boolean" :default _))
  (bind _keys (`BlueprintMapLibrary.Map_Keys` (`self.Required Keys`)))
  (for (_ _array_index) _keys
    (if (not (`BlueprintMapLibrary.Map_Find` `Player keycards`))
      (break)))
  (if (== _array_index (`KismetArrayLibrary.Array_LastIndex` _keys))
    (set `self.Allow Action` true)))

(fn `Return Is Blocker`
  (returns (NewParam :type Boolean))
  (return false))

(fn `Return keycard Object`
  (returns (`Keycard Level` :type "/Game/Blueprints/Keycard/keycardAccessLevel Enum"))
  (return "NewEnumerator0"))

(fn `UserConstructionScript`
  (bind _spline (`self.Spline`))
  (`|ExecutionSequence`
    (:`then_0`
      (`/Engine/EditorBlueprintResources/StandardMacros.IsValid` (`self.Activate Object`)
        (:`Is Valid`
          (`SplineComponent.SetLocationAtSplinePoint` _spline 1 (`self.K2_GetActorLocation` (`self.Activate Object`)) "World" true))
        (:`Is Not Valid`
          (`SplineComponent.SetLocationAtSplinePoint` _spline 1 (0.0 0.0 0.0) "Local" true))))))