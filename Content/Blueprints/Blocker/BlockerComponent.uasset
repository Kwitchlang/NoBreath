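; Blocker Blueprint for a barrier with four states (Locked, Unlocked, Shield, Off) that set mesh color, collision and visibility.
; The construction script applies the initial state, and ActivateObject switches to ActionState using the same duplicated logic, creating a dynamic material instance each time.
; Locked and Unlocked are solid, Shield is visible without collision, and Off is hidden without collision.
; A query reports teleport as blocked in every state except Unlocked, including Off.
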(event `/Game/Blueprints/Systems/PlayerInterface.ActivateObject`
  (bind _staticmesh (`self.StaticMesh`))
  (bind _staticmesh_2 (`self.StaticMesh`))
  (bind _staticmesh_3 (`self.StaticMesh`))
  (`KismetSystemLibrary.PrintString` "Activate Object called")
  (bind _output_get (set `self.Current StateState` (`self.ActionState`)))
  (switch `/Game/Blueprints/Blocker/BlockerState` _output_get
    (:`NewEnumerator0`
      (bind _returnvalue (`PrimitiveComponent.CreateDynamicMaterialInstance` _staticmesh_2 0 null))
      (`MaterialInstanceDynamic.SetVectorParameterValue` _returnvalue "Color" (struct :`R` 1.0 :`G` 0.018187 :`A` 1.0))
      (`PrimitiveComponent.SetCollisionEnabled` _staticmesh_3 "QueryAndPhysics")
      (`SceneComponent.SetVisibility` _staticmesh_3 true true))
    (:`NewEnumerator4`
      (bind _returnvalue_2 (`PrimitiveComponent.CreateDynamicMaterialInstance` _staticmesh_2 0 null))
      (`MaterialInstanceDynamic.SetVectorParameterValue` _returnvalue_2 "Color" (struct :`R` 0.48409 :`G` 1.0 :`B` 0.310215 :`A` 1.0))
      (`PrimitiveComponent.SetCollisionEnabled` _staticmesh_3 "QueryAndPhysics")
      (`SceneComponent.SetVisibility` _staticmesh_3 true true))
    (:`NewEnumerator1`
      (bind _returnvalue_3 (`PrimitiveComponent.CreateDynamicMaterialInstance` (`self.StaticMesh`) 0 null))
      (`MaterialInstanceDynamic.SetVectorParameterValue` _returnvalue_3 "Color" (struct :`G` 0.476947 :`B` 1.0 :`A` 1.0))
      (`PrimitiveComponent.SetCollisionEnabled` _staticmesh "NoCollision")
      (`SceneComponent.SetVisibility` _staticmesh true true))
    (:`NewEnumerator2`
      (bind _returnvalue_4 (`PrimitiveComponent.CreateDynamicMaterialInstance` _staticmesh_2 0 null))
      (`MaterialInstanceDynamic.SetVectorParameterValue` _returnvalue_4 "Color" (struct :`R` 1.0 :`G` 1.0 :`B` 1.0 :`A` 1.0))
      (`PrimitiveComponent.SetCollisionEnabled` _staticmesh_3 "NoCollision")
      (`SceneComponent.SetVisibility` (`self.StaticMesh`) false false))))

(fn `Return keycard Object`)

(fn `Return Teleport Through Blocker`
  (returns (`IS valid Object` :type Boolean))
  (locals (`Block Teleport` :type Boolean))
  (`|ExecutionSequence`
    (:`then_0`
      (switch `/Game/Blueprints/Blocker/BlockerState` (`self.Current StateState`)
        (:`NewEnumerator0`
          (set `local.Block Teleport` true))
        (:`NewEnumerator4`
          (set `local.Block Teleport` false))
        (:`NewEnumerator1`
          (set `local.Block Teleport` true))
        (:`NewEnumerator2`
          (set `local.Block Teleport` true))))
    (:`then_1`
      (return (`local.Block Teleport`)))))

(fn `UserConstructionScript`
  (bind _staticmesh (`self.StaticMesh`))
  (bind _staticmesh_2 (`self.StaticMesh`))
  (bind _staticmesh_3 (`self.StaticMesh`))
  (switch `/Game/Blueprints/Blocker/BlockerState` (`self.Current StateState`)
    (:`NewEnumerator0`
      (bind _returnvalue (`PrimitiveComponent.CreateDynamicMaterialInstance` _staticmesh_2 0 null))
      (`MaterialInstanceDynamic.SetVectorParameterValue` _returnvalue "Color" (struct :`R` 1.0 :`G` 0.018187 :`A` 1.0))
      (`PrimitiveComponent.SetCollisionEnabled` _staticmesh_3 "QueryAndPhysics")
      (`SceneComponent.SetVisibility` _staticmesh_3 true true))
    (:`NewEnumerator4`
      (bind _returnvalue_2 (`PrimitiveComponent.CreateDynamicMaterialInstance` _staticmesh_2 0 null))
      (`MaterialInstanceDynamic.SetVectorParameterValue` _returnvalue_2 "Color" (struct :`R` 0.48409 :`G` 1.0 :`B` 0.310215 :`A` 1.0))
      (`PrimitiveComponent.SetCollisionEnabled` _staticmesh_3 "QueryAndPhysics")
      (`SceneComponent.SetVisibility` _staticmesh_3 true true))
    (:`NewEnumerator1`
      (bind _returnvalue_3 (`PrimitiveComponent.CreateDynamicMaterialInstance` (`self.StaticMesh`) 0 null))
      (`MaterialInstanceDynamic.SetVectorParameterValue` _returnvalue_3 "Color" (struct :`G` 0.476947 :`B` 1.0 :`A` 1.0))
      (`PrimitiveComponent.SetCollisionEnabled` _staticmesh "NoCollision")
      (`SceneComponent.SetVisibility` _staticmesh true true))
    (:`NewEnumerator2`
      (bind _returnvalue_4 (`PrimitiveComponent.CreateDynamicMaterialInstance` _staticmesh_2 0 null))
      (`MaterialInstanceDynamic.SetVectorParameterValue` _returnvalue_4 "Color" (struct :`R` 1.0 :`G` 1.0 :`B` 1.0 :`A` 1.0))
      (`PrimitiveComponent.SetCollisionEnabled` _staticmesh_3 "NoCollision")
      (`SceneComponent.SetVisibility` (`self.StaticMesh`) false false))))