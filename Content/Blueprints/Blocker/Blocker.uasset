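; Blocker is an obstacle actor that disappears when activated.
; ActivateObject hides its static mesh, including child components, and disables the mesh's collision.
; The construction script creates a dynamic material instance and feeds the NonStatic variable into its "Non-Static" scalar parameter.
; ReturnIsBlocker identifies it as a blocker by returning true, while ReturnKeycardObject is left empty.
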(event `/Game/Blueprints/Systems/PlayerInterface.ActivateObject`
  (`SceneComponent.SetVisibility` (`self.StaticMesh`) false true)
  (`PrimitiveComponent.SetCollisionEnabled` (`self.StaticMesh`) "NoCollision"))

(fn `Return Is Blocker`
  (returns (NewParam :type Boolean))
  (return true))

(fn `Return keycard Object`)

(fn `UserConstructionScript`
  (bind _returnvalue (`PrimitiveComponent.CreateDynamicMaterialInstance` (`self.StaticMesh`) 0 null))
  (`MaterialInstanceDynamic.SetScalarParameterValue` _returnvalue "Non-Static" (`KismetMathLibrary.Conv_BoolToDouble` (`self.NonStatic`))))