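; Keycard actor that displays a door code and a vault code and carries an access level.
; On construction and BeginPlay, it reads both keycodes from the class defaults of its assigned keycode data and writes them as ungrouped numbers to two text elements.
; Query functions report its access type as the keycard level and return false for teleporting through blockers.
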(event `self.ReceiveBeginPlay`
  (`self.Update Keycard`))

(fn `Return keycard Object`
  (returns (`Keycard Level` :type "/Game/Blueprints/Keycard/KeycardColor Enum") (Executed :type Boolean))
  (return (`self.Access Type`) true))

(fn `Return Teleport Through Blocker`
  (returns (`IS valid Object` :type Boolean))
  (return false))

(fn `Update Keycard`
  (bind (_door_keycode _vault_keycode) (defaults `/Game/Blueprints/Keycard/keycard` (`self.Keycode Assiged Data`)))
  (`TextRenderComponent.K2_SetText` (`self.Door Code`) (`KismetTextLibrary.Conv_IntToText` _door_keycode false false))
  (`TextRenderComponent.K2_SetText` (`self.Vault Code`) (`KismetTextLibrary.Conv_IntToText` _vault_keycode false false)))

(fn `UserConstructionScript`
  (`self.Update Keycard`))