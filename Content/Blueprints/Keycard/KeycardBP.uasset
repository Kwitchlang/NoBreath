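; Keycard actor that shows a widget while a ThirdPersonCharacter stands inside its collision volume; no pickup logic is present.
; Overlap events store or clear the overlapping actor, and Tick casts it to toggle the widget's visibility.
; While the character is in range, Tick also runs a debug-drawn Visibility trace from the mesh to the character, but the hit result drives nothing.
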(event `self.ReceiveBeginPlay`
  (`SceneComponent.SetVisibility` (`self.Widget`) false true))

(event `self.ReceiveTick`
  (params (DeltaSeconds :type "Float (single-precision)"))
  (bind _overlapped_character (`self.Overlapped Character`))
  (bind _widget (`self.Widget`))
  (`/Engine/EditorBlueprintResources/StandardMacros.IsValid` _overlapped_character
    (:`Is Valid`
      (bind _asthird_person_character (cast `/Game/Blueprints/ThirdPersonCharacter/ThirdPersonCharacter` _overlapped_character)
        (:`then`
          (`SceneComponent.SetVisibility` _widget true true)
          (bind (_outhit _returnvalue) (`KismetSystemLibrary.LineTraceSingle` :`Start` (`SceneComponent.K2_GetComponentLocation` (`self.StaticMesh`)) :`End` (`self.K2_GetActorLocation` _asthird_person_character) :`TraceChannel` "TraceTypeQuery1" :`DrawDebugType` "ForOneFrame"))
          (if _returnvalue
            _))
        (:`CastFailed`
          (`SceneComponent.SetVisibility` _widget false true))))))

(event `self.Collision.OnComponentBeginOverlap`
  (params (OverlappedComponent :type "PrimitiveComponent Object Reference") (OtherActor :type "Actor Object Reference") (OtherComp :type "PrimitiveComponent Object Reference") (OtherBodyIndex :type Integer) (bFromSweep :type Boolean) (SweepResult :type "HitResult Structure (by ref)"))
  (set `self.Overlapped Character` OtherActor))

(event `self.Collision.OnComponentEndOverlap`
  (params (OverlappedComponent :type "PrimitiveComponent Object Reference") (OtherActor :type "Actor Object Reference") (OtherComp :type "PrimitiveComponent Object Reference") (OtherBodyIndex :type Integer))
  (set `self.Overlapped Character` null)
  (`SceneComponent.SetVisibility` (`self.Widget`) false true))

(fn `UserConstructionScript`)