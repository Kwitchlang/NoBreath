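; Procedural spline corridor that reports whether its environment is hazardous and how fast it drains oxygen.
; Construction builds a spline mesh per segment from MeshesInSpline, appending random picks from RandomMeshList when an entry is invalid.
; CorridoreState sets the hazard flag and oxygen rate, refreshed every Tick; AuthorityActivateObject restores it to Pressurized.
; Emissive warning-light code is disconnected, and GenerateStaticList, behind RandomizeSplineMesh, does nothing.
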(event `self.ReceiveBeginPlay`
  (`self.Set Enviornment State` :!label _label))

(event `self.ReceiveTick`
  (params (DeltaSeconds :type "Float (single-precision)"))
  (goto _label))

(event `Randomize Spline Mesh`
  (`self.Generate Static List`))

(event `/Game/Blueprints/Systems/Interfaces/AuthoritiveInterface.Authority Activate Object`
  (set `self.Corridore State` "NewEnumerator0"))

(fn `[Construction] Update Spline Meshes`
  (params (`Spline Comopnent` :type "SplineMeshComponent Object Reference (by ref)") (`Seslect from List` :type Integer))
  (returns (Mesh :type "StaticMesh Object Reference"))
  (locals (`Current Array` :type "Array of StaticMesh Object Reference"))
  (bind _spline_component__and_mesh_map (`self.Spline Component  and Mesh Map`))
  (`BlueprintMapLibrary.Map_Add` _spline_component__and_mesh_map `Spline Comopnent` (`|GetArrayItem` (`self.Meshes in Spline`) `Seslect from List`))
  (bind _values (`BlueprintMapLibrary.Map_Values` _spline_component__and_mesh_map))
  (bind _output (`|GetArrayItem` _values `Seslect from List`))
  (`/Engine/EditorBlueprintResources/StandardMacros.IsValid` _output
    (:`Is Valid`
      (return _output))
    (:`Is Not Valid`
      (`KismetArrayLibrary.Array_Add` (`self.Meshes in Spline`) (`/Game/Blueprints/Systems/CustomMacroLibrary.Get Random in Array` (`self.Random Mesh List`))))))

(fn `[Construction]Generate Mesh Spline`
  (locals (`Current Number` :type Integer))
  (bind _spline (`self.Spline`))
  (bind _meshes_in_spline (`self.Meshes in Spline`))
  (bind _returnvalue (`SplineComponent.GetNumberOfSplinePoints` _spline))
  (`BlueprintMapLibrary.Map_Clear` (`self.Spline Component  and Mesh Map`))
  (set `self.Current number of Splines` _returnvalue)
  (for _index (range (+ (- _returnvalue 2) 1))
    (`SplineComponent.SetSplinePointType` _spline _index (`self.Spline Type`) true)
    (bind _returnvalue_2 (`AddComponent|NODE_AddSplineMeshComponent-2`))
    (bind _mesh (`self.[Construction] Update Spline Meshes` _returnvalue_2 _index))
    (`StaticMeshComponent.SetStaticMesh` _returnvalue_2 _mesh)
    (`/Game/Blueprints/Systems/CustomMacroLibrary.Set Start and End Spline` (`self.Spline`) _index (`self.Coord Space`) _returnvalue_2)
    (`PrimitiveComponent.SetCollisionEnabled` _returnvalue_2 "QueryAndPhysics"))
  ;[1 1 1] Removes additional created meshes in array
  (bind _keys (`BlueprintMapLibrary.Map_Keys` (`self.Spline Component  and Mesh Map`)))
  (if (> (`KismetArrayLibrary.Array_Length` _meshes_in_spline) (`KismetArrayLibrary.Array_Length` _keys))
    (`KismetArrayLibrary.Array_Remove` _meshes_in_spline (`KismetArrayLibrary.Array_LastIndex` _meshes_in_spline))))

(fn `Generate Static List`)

(fn `Hazardous Enviornment`
  (returns (`Is Hazardous` :type Boolean) (`Decrease Oxygen Rate` :type "Float (double-precision)"))
  (return (`self.Enviorment NOT Safe`) (`self.Oxygen Decrease Variable`)))

(fn `Set Enviornment State`
  (switch `/Game/Blueprints/StructsEnums/CorridoreState` (`self.Corridore State`)
    (:`NewEnumerator0`
      (set `self.Enviorment NOT Safe` false))
    (:`NewEnumerator1`
      (set `self.Oxygen Decrease Variable` 2.0)
      (set `self.Enviorment NOT Safe` true :!label _label))
    (:`NewEnumerator2`
      (set `self.Oxygen Decrease Variable` 30.0)
      (goto _label))
    (:`NewEnumerator3`
      (set `self.Oxygen Decrease Variable` 30.0)
      (set `self.Enviorment NOT Safe` true))))

(fn `UserConstructionScript`
  (`self.[Construction]Generate Mesh Spline`)
  (`self.Set Enviornment State`))