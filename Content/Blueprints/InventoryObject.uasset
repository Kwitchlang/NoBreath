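; A pickup actor that places its stackable item type into the player's inventory when activated.
; ActivateObject passes StackableObject to AddToInventory on the game instance, then destroys the actor.
; BeginPlay switches on StackableObject to set the static mesh, with only the Breather Tank case wired.
; The construction script calls the parent's script and then ChangeMesh, which is empty here.
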(event `/Game/Blueprints/Systems/Interfaces/PlayerInteractableInterface.Activate Object`
  (`|ExecutionSequence`
    (:`then_0`
      (`/Game/Blueprints/Systems/CustomgameInstance.Add To Inventory` (`/Game/Blueprints/Systems/SystemFunctionLibrary.Game Instance Pure`) (`self.Stackable Object`)))
    (:`then_1`
      (`self.K2_DestroyActor`))))

(event `self.ReceiveBeginPlay`
  (switch `/Game/Blueprints/InteractableCLASS/inventoryType` (`self.Stackable Object`)
    (:`NewEnumerator0`
      (`StaticMeshComponent.SetStaticMesh` (`self.StaticMesh1`) "/Game/Assets/InteractableMesh/Breather_Tank.Breather_Tank"))))

(fn `Change Mesh`)

(fn `UserConstructionScript`
  (`parent.UserConstructionScript`)
  (`self.Change Mesh`))