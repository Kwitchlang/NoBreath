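; Space is an actor with a trigger component that toggles zero gravity on the third-person player character.
; When a ThirdPersonCharacter begins overlapping ActivateSpace, a nonzero gravity scale drops to zero and a forward velocity impulse along the capsule's facing sends the character drifting.
; If gravity is already near zero, the overlap restores normal gravity instead, so each entry flips the state.
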(event `self.Activate space.OnComponentBeginOverlap`
  (params (OverlappedComponent :type "PrimitiveComponent Object Reference") (OtherActor :type "Actor Object Reference") (OtherComp :type "PrimitiveComponent Object Reference") (OtherBodyIndex :type Integer) (bFromSweep :type Boolean) (SweepResult :type "HitResult Structure (by ref)"))
  (bind _asthird_person_character (cast `/Game/Blueprints/ThirdPersonCharacter/ThirdPersonCharacter` OtherActor))
  (bind _charactermovement (`Character.CharacterMovement` _asthird_person_character))
  (if (> (`CharacterMovementComponent.GravityScale` _charactermovement) 0.01)
    (set `CharacterMovementComponent.GravityScale` 0.0 _charactermovement)
    (`CharacterMovementComponent.AddImpulse` (`Character.CharacterMovement` _asthird_person_character) (* (`SceneComponent.GetForwardVector` (`Character.CapsuleComponent` _asthird_person_character)) 100.0) true)
    (else
      (set `CharacterMovementComponent.GravityScale` 1.0 _charactermovement))))

(fn `UserConstructionScript`)