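; Door control panel actor that presents a keypad for entering a passcode.
; At BeginPlay it creates a DoorKeypadUI widget with its Passcode and a self reference, displayed through its Widget component.
; Activating the panel blends the player's view to it and sets mouse visibility with focus on the keypad.
; ActivateObjectsfromUI sends an authority activation message to each object in its ActivateObjects list.
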(event `/Game/Blueprints/Systems/Interfaces/PlayerInteractableInterface.Activate Object`
  (`PlayerController.SetViewTargetWithBlend` (`GameplayStatics.GetPlayerController` 0) self 0.3 "VTBlend_EaseInOut" 1.0 false)
  (`/Game/Blueprints/Systems/SystemFunctionLibrary.Set Mouse Visability` "NewEnumerator0" (`self.Keypad UI `)))

(event `self.ReceiveBeginPlay`
  (bind _returnvalue (`|CreateWidget` "/Game/Blueprints/UI/DiageticUI/DoorKeypadUI.DoorKeypadUI_C" null self (`self.Passcode`)))
  (`WidgetComponent.SetWidget` (`self.Widget`) _returnvalue))

(event `Activate Objects from UI`
  (for _array_element (`self.Activate Objects`)
    (message `/Game/Blueprints/Systems/Interfaces/AuthoritiveInterface.Authority Activate Object` _array_element)))

(fn `UserConstructionScript`)