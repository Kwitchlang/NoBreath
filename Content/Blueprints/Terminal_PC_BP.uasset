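; An interactable PC terminal that, when activated, blends the player's view to itself and changes mouse visibility.
; On BeginPlay it puts a TerminalUI in its widget component and creates a TerminalEntry child widget for each system tool in TerminalStruct.
; The construction script draws splines from the terminal to every actor each tool uses, stepping the start point down per tool to visualize the links.
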(event `/Game/Blueprints/Systems/Interfaces/PlayerInteractableInterface.Activate Object`
  (`PlayerController.SetViewTargetWithBlend` (`GameplayStatics.GetPlayerController` 0) self 0.3 "VTBlend_EaseInOut" 1.0 false)
  (`/Game/Blueprints/Systems/SystemFunctionLibrary.Set Mouse Visability` "NewEnumerator0"))

(event `self.ReceiveBeginPlay`
  (bind (_terminal_struct_username _terminal_struct_password _terminal_struct_terminalname _terminal_struct_terminalsystemtools) (break `/Game/Blueprints/StructsEnums/TerminalStruct` (`self.Terminal Struct`)))
  (bind _returnvalue (`|CreateWidget` "/Game/Blueprints/UI/DiageticUI/Terminal/TerminalUI.TerminalUI_C"))
  (bind _output_get (set `self.Termnal UI` _returnvalue))
  (`WidgetComponent.SetWidget` (`self.Widget`) _output_get)
  (for _array_element _terminal_struct_terminalsystemtools
    (bind _returnvalue_2 (`|CreateWidget` "/Game/Blueprints/UI/DiageticUI/Terminal/TerminalEntry.TerminalEntry_C" null _array_element))
    (`PanelWidget.AddChild` _returnvalue_2)))

(fn `UserConstructionScript`
  (bind (_terminal_struct_username _terminal_struct_password _terminal_struct_terminalname _terminal_struct_terminalsystemtools) (break `/Game/Blueprints/StructsEnums/TerminalStruct` (`self.Terminal Struct`)))
  (bind (_relativelocation_x _relativelocation_y _relativelocation_z) (`KismetMathLibrary.BreakVector` (`SceneComponent.RelativeLocation` (`self.Construction Location`))))
  (for (_array_element _array_index) _terminal_struct_terminalsystemtools
    (for _array_element_2 (`.ObjecttoUse_6_544EF8F748CF693D81EE1EB93E1A5603` (break `/Game/Blueprints/StructsEnums/TerminalEntryStrut` _array_element))
      (bind _returnvalue (`AddComponent|NODE_AddSplineComponent-0`))
      (`SplineComponent.SetLocationAtSplinePoint` _returnvalue 0 (`KismetMathLibrary.MakeVector` _relativelocation_x _relativelocation_y (+ _relativelocation_z (* _array_index -8.0))) "Local" true)
      (`SplineComponent.SetLocationAtSplinePoint` _returnvalue 1 (`self.K2_GetActorLocation` _array_element_2) "World" true))))