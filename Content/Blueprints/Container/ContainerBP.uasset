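; ContainerBP is a rotatable container with Blocker child actors that can be turned in 90-degree steps or reset to zero rotation.
; Tick eases the Container component toward ZRotation with RInterpTo, using a fixed delta time, while ActivateObject only stores the current rotation.
; The construction script sets each child Blocker's type from the BlockerType array.
; Two query functions return a fixed keycard level and disallow teleporting through blockers.
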(event `/Game/Blueprints/Systems/PlayerInterface.ActivateObject`
  (set `self.Current Rotation` (`SceneComponent.RelativeRotation` (`self.Container`))))

(event `self.ReceiveTick`
  (params (DeltaSeconds :type "Float (single-precision)"))
  (bind _container (`self.Container`))
  (`SceneComponent.K2_SetRelativeRotation` _container (`KismetMathLibrary.RInterpTo` (`SceneComponent.RelativeRotation` _container) (`KismetMathLibrary.MakeRotator` 0.0 0.0 (`self.z Rotation`)) 1.0 0.01) false false))

(event `Rotate Object Right`
  (bind _container (`self.Container`))
  (`SceneComponent.K2_SetRelativeRotation` _container (`KismetMathLibrary.ComposeRotators` (`SceneComponent.RelativeRotation` _container) (struct :`Yaw` 90.0)) false false))

(event `Rotate Object Left`
  (bind _container (`self.Container`))
  (`SceneComponent.K2_SetRelativeRotation` _container (`KismetMathLibrary.ComposeRotators` (`SceneComponent.RelativeRotation` _container) (struct :`Yaw` -90.0)) false false))

(event `Reset`
  (`SceneComponent.K2_SetRelativeRotation` :`self` (`self.Container`)))

(fn `Return keycard Object`
  (returns (`Keycard Level` :type "/Game/Blueprints/Keycard/KeycardColor Enum") (Executed :type Boolean))
  (return "NewEnumerator1" false))

(fn `Return Teleport Through Blocker`
  (returns (`IS valid Object` :type Boolean))
  (return false))

(fn `UserConstructionScript`
  (for (_array_element _array_index) (`|MakeArray` (`self.Blocker -x Actor`) (`self.Blocker +x`) (`self.Blocker -y`) (`self.Blocker +y`))
    (bind _asblocker (cast `/Game/Blueprints/Blocker/Blocker` (`ChildActorComponent.ChildActor` _array_element)))
    (`/Game/Blueprints/Blocker/Blocker.Change Type` _asblocker (`|GetArrayItem` (`self.Blocker Type`) _array_index))))