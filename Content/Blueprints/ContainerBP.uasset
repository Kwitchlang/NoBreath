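; ContainerBP is a container Blueprint that configures child Blocker actors when it is constructed.
; Its construction script loops over a four-entry list of child actor components, in which Blockery appears twice, and casts each child to Blocker.
; Each Blocker receives a ChangeType call with the BlockerType element at the same index.
; BeginPlay is empty, so all logic lives in construction.
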(event `self.ReceiveBeginPlay`)

(fn `UserConstructionScript`
  (for (_array_element _array_index) (`|MakeArray` (`self.Blocker -x Actor`) (`self.Blocker +x`) (`self.Blocker -y`) (`self.Blocker +y`))
    (bind _asblocker (cast `/Game/UsedBlueprints/Blocker` (`ChildActorComponent.ChildActor` _array_element)))
    (`/Game/UsedBlueprints/Blocker.Change Type` _asblocker (`|GetArrayItem` (`self.Blocker Type`) _array_index))))