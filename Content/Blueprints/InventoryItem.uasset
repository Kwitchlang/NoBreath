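; InventoryItem is a pickup actor that puts an item into the player's inventory when activated.
; Its ActivateObject event passes the item's InventoryType to AddToInventory on the game instance, then destroys the actor.
; Inventory storage is delegated to the game instance, and the actor has no active BeginPlay, overlap or Tick logic.
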(event `/Game/Blueprints/Systems/Interfaces/PlayerInteractableInterface.Activate Object`
  (`|ExecutionSequence`
    (:`then_0`
      (`/Game/Blueprints/Systems/CustomgameInstance.Add To Inventory` (`/Game/Blueprints/Systems/SystemFunctionLibrary.Game Instance Pure`) (`self.Inventory Type`)))
    (:`then_1`
      (`self.K2_DestroyActor`))))

(fn `UserConstructionScript`
  (`parent.UserConstructionScript`))