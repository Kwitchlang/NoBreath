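; Moving platform that steps through an array of relative locations when activated.
; ActivateObject advances the index by the switch method (clamp at end, loop to start or ping-pong), sets the target, then re-triggers after a delay while repeat is on.
; Tick eases the platform toward the target with VInterpTo on a fixed delta time, so speed depends on frame rate.
; BreakEvent stops repeating; keycard and teleport-blocker functions return fixed values.
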(event `self.ReceiveTick`
  (params (DeltaSeconds :type "Float (single-precision)"))
  (bind _platform (`self.Platform`))
  (`SceneComponent.K2_SetRelativeLocation` _platform (`KismetMathLibrary.VInterpTo` (`SceneComponent.RelativeLocation` _platform) (`self.Target Location`) 1.0 0.01) false false))

(event `Activate Object`
  (bind _location_select (`self.Location Select`))
  (bind _returnvalue (`KismetArrayLibrary.Array_LastIndex` (`self.Location Array`)))
  (bind _returnvalue_2 (- (`self.Location Select`) 1))
  (bind _returnvalue_3 (+ _location_select 1))
  (bind _returnvalue_4 (+ (`self.Location Select`) 1))
  (switch `/Game/Blueprints/MultifacetPanel/Actiontype` "NewEnumerator0" :!label _label
    (:`NewEnumerator0`
      (`|ExecutionSequence`
        (:`then_0`
          (switch `/Game/Blueprints/MultifacetPanel/method` (`self.SwitchMethod`)
            (:`NewEnumerator0`
              (set `self.Location Select` (`KismetMathLibrary.Clamp` _returnvalue_4 0 _returnvalue)))
            (:`NewEnumerator2`
              (if (> _returnvalue_4 _returnvalue)
                (set `self.Location Select` 0)
                (else
                  (set `self.Location Select` _returnvalue_4))))
            (:`NewEnumerator1`
              (if (`self.Backwards`)
                (if (< _returnvalue_2 0)
                  (set `self.Backwards` false)
                  (set `self.Location Select` (+ (`self.Location Select`) 1))
                  (else
                    (set `self.Location Select` _returnvalue_2)))
                (elif (> _returnvalue_3 (`KismetArrayLibrary.Array_LastIndex` (`self.Location Array`)))
                  (set `self.Backwards` true)
                  (set `self.Location Select` (- _location_select 1))
                  (else
                    (set `self.Location Select` _returnvalue_3)))))))
        (:`then_1`
          (set `self.Target Location` (`|GetArrayItem` (`self.Location Array`) (`self.Location Select`))))
        (:`then_2`
          (`KismetSystemLibrary.Delay` (`self.Delay`))
          (if (`self.Repeate`)
            (`self.ActivateObject`)))))))

(event `self.ActivateObject`
  (goto _label))

(event `Break Event`
  (set `self.Repeate` false))

(fn `Return keycard Object`
  (returns (`Keycard Level` :type "/Game/Blueprints/Keycard/keycardAccessLevel Enum") (Executed :type Boolean))
  (return "NewEnumerator0" false))

(fn `Return Teleport Through Blocker`
  (returns (`IS valid Object` :type Boolean))
  (return false))

(fn `UserConstructionScript`)