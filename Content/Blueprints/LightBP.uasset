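; Light actor Blueprint that starts a rect light at a default intensity and switches it to a fixed bright level when activated through AuthorityActivateObject.
; Activation also sets a BreakLoop flag meant to end a flicker loop.
; That loop, which randomizes light intensity and a dynamic material's Intensity parameter at random delays, is disconnected from any event and never runs.
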(event `self.ReceiveBeginPlay`
  (`LightComponent.SetIntensity` (`self.RectLight`) (`self.Default Intensity`)))

(event `/Game/Blueprints/Systems/Interfaces/AuthoritiveInterface.Authority Activate Object`
  (set `self.Break Loop` true)
  (`LightComponent.SetIntensity` (`self.RectLight`) 600.0))

(fn `UserConstructionScript`)