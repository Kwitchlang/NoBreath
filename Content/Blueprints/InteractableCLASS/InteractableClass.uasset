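; Base interactable actor that shows a "[E]" prompt widget when the player is nearby and in line of sight.
; A collision component tracks the overlapping actor and hides the prompt when the overlap ends.
; While overlapped, Tick line-traces on the Camera channel toward that character and toggles visibility by whether it hits the GameInstance's player character.
; No input or interaction logic is present, and component hits only print a debug string.
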(event `self.ReceiveBeginPlay`
  (`SceneComponent.SetVisibility` (`self.Interaction Widget`) false true)
  (bind _returnvalue (`|CreateWidget` "/Game/Blueprints/UI/DiageticUI/PressInteractUI.PressInteractUI_C" null (`KismetTextLibrary.Conv_StringToText` "[E]")))
  (`WidgetComponent.SetWidget` (`self.Interaction Widget`) _returnvalue))

(event `self.ReceiveTick`
  (params (DeltaSeconds :type "Float (single-precision)"))
  (`/Engine/EditorBlueprintResources/StandardMacros.IsValid` (`self.Overlapped Character`)
    (:`Is Valid`
      (bind (_outhit _returnvalue) (`KismetSystemLibrary.LineTraceSingle` (`self.K2_GetActorLocation`) (`self.K2_GetActorLocation` (`self.Overlapped Character`)) "TraceTypeQuery2"))
      (if _returnvalue
        (bind _output_get (set `self.Linetrace connecting with player` (== (`.HitActor` (`GameplayStatics.BreakHitResult` _outhit)) (`/Game/Blueprints/Systems/CustomgameInstance.Player character` (`/Game/Blueprints/Systems/SystemFunctionLibrary.Game Instance Pure`)))))
        (if _output_get
          (bind _newparam2 (`/Game/Blueprints/Systems/CustomMacroLibrary.Exec to Bool` :!label _label)
            (:`Exec`
              (`SceneComponent.SetVisibility` (`self.Interaction Widget`) _newparam2 true)))
          (else
            (goto _label :!via `False`)))))))

(event `self.Player Collision Detection.OnComponentBeginOverlap`
  (params (OverlappedComponent :type "PrimitiveComponent Object Reference") (OtherActor :type "Actor Object Reference") (OtherComp :type "PrimitiveComponent Object Reference") (OtherBodyIndex :type Integer) (bFromSweep :type Boolean) (SweepResult :type "HitResult Structure (by ref)"))
  (set `self.Overlapped Character` OtherActor))

(event `self.Player Collision Detection.OnComponentEndOverlap`
  (params (OverlappedComponent :type "PrimitiveComponent Object Reference") (OtherActor :type "Actor Object Reference") (OtherComp :type "PrimitiveComponent Object Reference") (OtherBodyIndex :type Integer))
  (set `self.Overlapped Character` null)
  (`SceneComponent.SetVisibility` (`self.Interaction Widget`) false true))

(event `self.Player Collision Detection.OnComponentHit`
  (params (HitComponent :type "PrimitiveComponent Object Reference") (OtherActor :type "Actor Object Reference") (OtherComp :type "PrimitiveComponent Object Reference") (NormalImpulse :type "Vector Structure") (Hit :type "HitResult Structure (by ref)"))
  (`KismetSystemLibrary.PrintString` "Collider hit"))

(fn `UserConstructionScript`)