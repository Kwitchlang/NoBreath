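; FuseBox is an activatable Blueprint that fires a radial physics impulse through its RadialForce component.
; ActivateObject and Fireimpulse share one path, which fires the impulse and only afterwards reapplies the radius, force and impulse strength variables.
; The construction script also copies those variables onto the component.
; The keycard getter is an empty stub, and the teleport-through-blocker query returns false.
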(event `Fireimpulse`
  (bind _radialforce (`self.RadialForce`))
  (`RadialForceComponent.FireImpulse` (`self.RadialForce`) :!label _label)
  (set `RadialForceComponent.Radius` (`self.Radius Explosion`) _radialforce)
  (set `RadialForceComponent.ForceStrength` (`self.Force Strength`) _radialforce)
  (set `RadialForceComponent.ImpulseStrength` (`self.Impulse Strength`) _radialforce))

(event `/Game/Blueprints/Systems/PlayerInterface.ActivateObject`
  (goto _label))

(fn `Return keycard Object`)

(fn `Return Teleport Through Blocker`
  (returns (`IS valid Object` :type Boolean))
  (return false))

(fn `UserConstructionScript`
  (bind _radialforce (`self.RadialForce`))
  (set `RadialForceComponent.Radius` (`self.Radius Explosion`) _radialforce)
  (set `RadialForceComponent.ForceStrength` (`self.Force Strength`) _radialforce)
  (set `RadialForceComponent.ImpulseStrength` (`self.Impulse Strength`) _radialforce))