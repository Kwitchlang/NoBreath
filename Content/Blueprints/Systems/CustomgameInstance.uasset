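; Custom game instance that serves as a central hub for UI screens, main level loading and session flags.
; Events create and show splash, menu, settings, exit, ESC and interaction widgets, reusing only the settings widget.
; A log widget starts hidden, receives name/text entries as children and toggles visibility through a FlipFlop.
; Helper events blend the camera back to the player, adjust mouse visibility and store a Landscape reference.
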(event `Load Main Level`
  ;[1 1 1] Load main level
  (`GameplayStatics.OpenLevel` "PrototypeLevel001_2")
  (set `self.In Game Session` true))

(event `Program EXE Started`
  ;[1 1 1] Program Started
  (set `self.Game EXE Started` true))

(event `Show Splash Screen`
  ;[1 1 1] Show Splash Screen
  (bind _returnvalue (`|CreateWidget` "/Game/Blueprints/UI/Menu_UI/01_SplashScreen.01_SplashScreen_C"))
  (bind _output_get (set `self.Splash Screen UI` _returnvalue))
  (`UserWidget.AddToViewport` _output_get 0))

(event `Show Main menu`
  ;[1 1 1] Show Main Menu
  (bind _returnvalue (`|CreateWidget` "/Game/Blueprints/UI/Menu_UI/02_MainMenu.02_MainMenu_C" (`GameplayStatics.GetPlayerController` 0)))
  (bind _output_get (set `self.Main Menu UI` _returnvalue))
  (`UserWidget.AddToViewport` _output_get 0))

(event `Show Options`
  ;[1 1 1] Show Options Menu
  (`/Engine/EditorBlueprintResources/StandardMacros.IsValid` (`self.Settings UI`)
    (:`Is Valid`
      _)
    (:`Is Not Valid`
      (bind _returnvalue (`|CreateWidget` "/Game/Blueprints/UI/Menu_UI/03_Settings.03_Settings_C"))
      (bind _output_get (set `self.Settings UI` _returnvalue))))
  (`UserWidget.AddToViewport` _output_get 0))

(event `Show Exit Screen`
  ;[1 1 1] Show Exit Screen
  (bind _returnvalue (`|CreateWidget` "/Game/Blueprints/UI/Menu_UI/05_ExitMenu.05_ExitMenu_C"))
  (bind _output_get (set `self.Exit Menu UI` _returnvalue))
  (`UserWidget.AddToViewport` _output_get 0))

(event `Show ESC Menu`
  ;[1 1 1] Show ESC menu
  (bind _returnvalue (`|CreateWidget` "/Game/Blueprints/UI/Player_UI/02_PlayerESCMenu.02_PlayerESCMenu_C"))
  (bind _output_get (set `self.ESC Wirdget` _returnvalue))
  (`UserWidget.AddToViewport` _output_get 0)
  (set `PlayerController.bShowMouseCursor` true (`GameplayStatics.GetPlayerController` 0)))

(event `Project to Screen`
  (params (Name :type Text) (log :type Text))
  (bind _returnvalue (`|CreateWidget` "/Game/Blueprints/UI/Player_UI/InventoryUI/InteractedUI.InteractedUI_C" null Name log))
  (`UserWidget.AddToViewport` _returnvalue 0))

(event `Add to Log Entry`
  (params (`Name ` :type Text) (Blog :type Text))
  (bind _log_ui (`self.Log UI`))
  (bind _returnvalue (`|CreateWidget` "/Game/Blueprints/UI/Player_UI/InventoryUI/LogEntry.LogEntry_C" (`GameplayStatics.GetPlayerController` 0) `Name ` Blog))
  (`/Engine/EditorBlueprintResources/StandardMacros.IsValid` _log_ui
    (:`Is Valid`
      (`PanelWidget.AddChild` (`/Game/Blueprints/UI/Player_UI/InventoryUI/LogUI.ContentsBox` _log_ui) _returnvalue))))

(event `Show Log Entries`
  (bind _log_ui (`self.Log UI`))
  (`/Engine/EditorBlueprintResources/StandardMacros.FlipFlop`
    (:`A`
      (`Widget.SetVisibility` _log_ui "Visible")
      (`/Game/Blueprints/Systems/SystemFunctionLibrary.Set Mouse Visability` "NewEnumerator0"))
    (:`B`
      (`Widget.SetVisibility` _log_ui "Hidden"))))

(event `Initialize UI`
  (bind _returnvalue (`|CreateWidget` "/Game/Blueprints/UI/Player_UI/InventoryUI/LogUI.LogUI_C"))
  (bind _output_get (set `self.Log UI` _returnvalue))
  (`UserWidget.AddToViewport` _output_get 0)
  (`Widget.SetVisibility` _output_get "Hidden"))

(event `Set Camera`
  ;[1 1 1] Change Camera to player
  (`PlayerController.SetViewTargetWithBlend` (`GameplayStatics.GetPlayerController` 0) (`GameplayStatics.GetPlayerCharacter` 0) 0.5 "VTBlend_EaseInOut" 1.0 false)
  (`/Game/Blueprints/Systems/SystemFunctionLibrary.Set Mouse Visability` "NewEnumerator1"))

(event `Reference landscape`
  (params (landscape :type "Landscape Object Reference"))
  (set `self.landscape` landscape))