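; System function library of global helpers for game instance access, mouse input modes and UI text.
; It returns the game instance cast to CustomGameInstance, and toggles the first player's cursor between centered UI-only input with widget focus and hidden game-only input.
; A text helper hides and clears a text widget when its content is empty, otherwise setting it to the content wrapped in a prefix and suffix.
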(fn `Center Mouse`
  (bind (_returnvalue_x _returnvalue_y) (`KismetMathLibrary.BreakVector2D` (`WidgetLayoutLibrary.GetViewportSize` null)))
  (`PlayerController.SetMouseLocation` (`GameplayStatics.GetPlayerController` null) (`KismetMathLibrary.FTrunc` (/ _returnvalue_x 2.0)) (`KismetMathLibrary.FTrunc` (/ _returnvalue_y 2.0))))

(fn `Game Instance Pure`
  (returns (`Custome Game Instance` :type "/Game/Blueprints/Systems/CustomgameInstance Object Reference"))
  (bind _ascustom_game_instance (cast `/Game/Blueprints/Systems/CustomgameInstance` (`GameplayStatics.GetGameInstance` null)))
  (return _ascustom_game_instance))

(fn `Set Mouse Visability`
  (params (`Mouse Type` :type "/Game/Blueprints/Systems/SetUIMouseType Enum" :default "NewEnumerator0") (InWidgetToFocus :type "Widget Object Reference"))
  (bind _returnvalue (`GameplayStatics.GetPlayerController` null))
  (switch `/Game/Blueprints/Systems/SetUIMouseType` `Mouse Type`
    (:`NewEnumerator0`
      (set `PlayerController.bShowMouseCursor` true _returnvalue)
      (`self.Center Mouse` null)
      (`WidgetBlueprintLibrary.SetInputMode_UIOnlyEx` _returnvalue InWidgetToFocus))
    (:`NewEnumerator1`
      (set `PlayerController.bShowMouseCursor` false _returnvalue)
      (`WidgetBlueprintLibrary.SetInputMode_GameOnly` _returnvalue))))

(fn `Set Text Visibility by Content`
  (params (Precursor :type String) (Content :type Text) (Procursor :type String) (NewParam :type "TextBlock Object Reference"))
  (returns (String :type Text))
  (bind _returnvalue (`KismetTextLibrary.Conv_TextToString` Content))
  (bind _returnvalue_2 (`KismetTextLibrary.Conv_StringToText` (`KismetStringLibrary.Concat_StrStr` Precursor _returnvalue Procursor)))
  (if (`KismetStringLibrary.EqualEqual_StrStr` _returnvalue)
    (`Widget.SetVisibility` NewParam "Hidden")
    (`TextBlock.SetText` NewParam "")
    (return _returnvalue_2)
    (else
      (`TextBlock.SetText` NewParam _returnvalue_2))))